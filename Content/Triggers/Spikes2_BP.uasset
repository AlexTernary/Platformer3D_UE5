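; Spike trap hazard for the 3D platformer that ends the player's run on contact.
; On BeginPlay it caches the game mode, waits TimeOffset, then plays a timeline that moves DeathCollision along its ZMoving track, shifted down in Z.
; The delay lets separate instances start out of phase.
; When BP_ThirdPersonCharacter overlaps DeathCollision, it calls MOpenLevel on the game mode.
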(event `self.ReceiveBeginPlay`
  (bind _asplatformer_3dgame_mode_bp (cast `/Game/BP/Platformer3DGameMode_BP` (`GameplayStatics.GetGameMode`)))
  (set `self.As Platformer 3DGame Mode BP` _asplatformer_3dgame_mode_bp)
  (`KismetSystemLibrary.Delay` (`self.Time Offset`))
  (bind (_direction _z_moving) (`Timeline|Timeline`)
    (:`Update`
      (`SceneComponent.K2_SetRelativeLocation` (`self.DeathCollision`) (- _z_moving (0.0 0.0 50.0)) false false))))

(event `self.DeathCollision.OnComponentBeginOverlap`
  (params (OverlappedComponent :type "PrimitiveComponent Object Reference") (OtherActor :type "Actor Object Reference") (OtherComp :type "PrimitiveComponent Object Reference") (OtherBodyIndex :type Integer) (bFromSweep :type Boolean) (SweepResult :type "HitResult Structure (by ref)"))
  (cast `/Game/ThirdPerson/Blueprints/BP_ThirdPersonCharacter` OtherActor)
  (`/Game/BP/Platformer3DGameMode_BP.MOpen Level` (`self.As Platformer 3DGame Mode BP`)))

(fn `UserConstructionScript`)