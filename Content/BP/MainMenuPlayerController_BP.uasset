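; Player controller for the main menu that opens the menu on begin play and switches between the main menu, settings screen and level load.
; Menu events clear all widgets, then lazily create and cache each widget before adding it to the viewport.
; Opening the main menu also shows the cursor with Game-and-UI input, while level start loads LvlG after a short delay.
; Holding H temporarily hides the settings widget.
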(event `self.ReceiveBeginPlay`
  (`self.MOpenMainMenu`))

(event `MOpenLevel1`
  ;[1 1 1] Open Level 1
  (`KismetSystemLibrary.Delay` 0.2)
  (`GameplayStatics.OpenLevel` "LvlG"))

(event `MOpenMainMenu`
  ;[1 1 1] Open Main Menu
  (`WidgetLayoutLibrary.RemoveAllWidgets`)
  (`/Engine/EditorBlueprintResources/StandardMacros.IsValid` (`self.Main Menu WB`)
    (:`Is Valid`
      _)
    (:`Is Not Valid`
      (bind _returnvalue (`|CreateWidget` "/Game/WB/MainMenu_WB.MainMenu_WB_C"))
      (bind _output_get (set `self.Main Menu WB` _returnvalue))))
  (`UserWidget.AddToViewport` _output_get 0)
  (set `self.bShowMouseCursor` true)
  (`WidgetBlueprintLibrary.SetInputMode_GameAndUIEx` self (`self.Main Menu WB`) "LockInFullscreen"))

(event `MOpen Main Settings`
  ;[1 1 1] Opne Main Settigs
  (`WidgetLayoutLibrary.RemoveAllWidgets`)
  (`/Engine/EditorBlueprintResources/StandardMacros.IsValid` (`self.Settings WB`)
    (:`Is Valid`
      _)
    (:`Is Not Valid`
      (bind _returnvalue (`|CreateWidget` "/Game/WB/MainSettings_WB.MainSettings_WB_C"))
      (bind _output_get (set `self.Settings WB` _returnvalue))))
  (`UserWidget.AddToViewport` _output_get 0))

(event `Key|H`
  (params (Key :type "Key Structure"))
  (:`Pressed`
    (`/Engine/EditorBlueprintResources/StandardMacros.IsValid` (`self.Settings WB`)
      (:`Is Valid`
        (`Widget.RemoveFromParent` (`self.Settings WB`)))))
  (:`Released`
    (`/Engine/EditorBlueprintResources/StandardMacros.IsValid` (`self.Settings WB`)
      (:`Is Valid`
        (`UserWidget.AddToViewport` (`self.Settings WB`) 0)))))

(fn `UserConstructionScript`)