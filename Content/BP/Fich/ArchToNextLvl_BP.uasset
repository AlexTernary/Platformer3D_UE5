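; Level exit arch for a 3D platformer that opens the next level once the player has enough score.
; When the game mode signals max score achieved, the arch gains a shield overlay material and spawns a Niagara dust effect.
; A third-person character overlapping the collision with sufficient score intensifies that effect in two timed stages before the level change.
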(event `self.ReceiveBeginPlay`
  (bind _asplatformer_3dgame_mode_bp (cast `/Game/BP/Platformer3DGameMode_BP` (`GameplayStatics.GetGameMode`)))
  (add `/Game/BP/Platformer3DGameMode_BP.MaxScoreAchived` _asplatformer_3dgame_mode_bp (delegate `Activate backlight`)))

(event `Activate backlight`
  (bind _defaultsceneroot (`self.DefaultSceneRoot`))
  (`MeshComponent.SetOverlayMaterial` (`self.Arch`) "/Game/Materials/Effects/Inst_Arch_Shield.Inst_Arch_Shield")
  (bind _returnvalue (`NiagaraFunctionLibrary.SpawnSystemAtLocation` "/Game/FX/FX_Dust.FX_Dust" (+ (`SceneComponent.K2_GetComponentLocation` _defaultsceneroot) (0.0 0.0 160.0)) (`KismetMathLibrary.Conv_VectorToRotator` (`SceneComponent.GetForwardVector` _defaultsceneroot)) (0.7 0.1 1.9)))
  (set `self.FX_Dust` _returnvalue))

(event `self.Coll.OnComponentBeginOverlap`
  (params (OverlappedComponent :type "PrimitiveComponent Object Reference") (OtherActor :type "Actor Object Reference") (OtherComp :type "PrimitiveComponent Object Reference") (OtherBodyIndex :type Integer) (bFromSweep :type Boolean) (SweepResult :type "HitResult Structure (by ref)"))
  (bind _fx_dust (`self.FX_Dust`))
  (bind _asbp_third_person_character (cast `/Game/ThirdPerson/Blueprints/BP_ThirdPersonCharacter` OtherActor))
  (if (>= (`/Game/ThirdPerson/Blueprints/BP_ThirdPersonCharacter.CurrentScore` _asbp_third_person_character) (`self.ScoreToNextLevel`))
    (`NiagaraComponent.SetVariableFloat` _fx_dust "SpawnRate" 1000.0)
    (`NiagaraComponent.SetVariableFloat` _fx_dust "Scale" 100.0)
    (`KismetSystemLibrary.Delay` 3.0)
    (`NiagaraComponent.SetVariableFloat` _fx_dust "Scale" 150.0)
    (`KismetSystemLibrary.Delay` 2.0)
    (`GameplayStatics.OpenLevelBySoftObjectPtr` (`self.NextLevel`))))

(fn `UserConstructionScript`)