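; InvisBlock is an actor whose Block component is briefly revealed by a trigger call.
; ActivateInvis compares the incoming TriggerIndex with TriggerIndex, then unhides Block for two seconds before hiding it again.
; The AlreadyShow flag is never reset here, so the reveal happens only once.
; An unconnected "Show By distance" branch repeats the reveal based on the actor's distance from world origin, but never runs.
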(event `/Game/BP/Interfeces/InvisInter_BP.ActivateInvis`
  (params (TriggerIndex :type Integer))
  (bind _block (`self.Block`))
  (if (== TriggerIndex (`self.TriggerIndex`))
    (if (not (`self.AlreadyShow?`))
      (`SceneComponent.SetHiddenInGame` (`self.Block`) false false)
      (set `self.AlreadyShow?` true)
      (`SceneComponent.SetHiddenInGame` _block false false)
      (`KismetSystemLibrary.Delay` 2.0)
      (`SceneComponent.SetHiddenInGame` _block true false))))

(fn `UserConstructionScript`)