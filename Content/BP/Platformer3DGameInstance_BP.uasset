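; Game instance for a 3D platformer that creates and shows the main menu and settings widgets.
; Each event lazily creates its widget for the first player controller, caches it in a variable, and adds it to the viewport on each call.
; The main menu event also shows the mouse cursor and switches to UI-only input, focused on the menu with the mouse locked in fullscreen.
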(event `AddMainMenu_WB`
  (bind _returnvalue (`GameplayStatics.GetPlayerController` 0))
  ;[1 1 1] Main Menu WB
  (`/Engine/EditorBlueprintResources/StandardMacros.IsValid` (`self.Main Menu WB`)
    (:`Is Valid`
      _)
    (:`Is Not Valid`
      (bind _returnvalue_2 (`|CreateWidget` "/Game/WB/MainMenu_WB.MainMenu_WB_C" (`GameplayStatics.GetPlayerController` 0)))
      (bind _output_get (set `self.Main Menu WB` _returnvalue_2))))
  (`UserWidget.AddToViewport` _output_get 0)
  (`UserWidget.AddToViewport` (`self.Main Menu WB`) 0)
  (set `PlayerController.bShowMouseCursor` true _returnvalue)
  (`WidgetBlueprintLibrary.SetInputMode_UIOnlyEx` _returnvalue (`self.Main Menu WB`) "LockInFullscreen"))

(event `Open Settings`
  (`/Engine/EditorBlueprintResources/StandardMacros.IsValid` (`self.Option WB`)
    (:`Is Valid`
      _)
    (:`Is Not Valid`
      (bind _returnvalue (`|CreateWidget` "/Game/WB/Settings_WB.Settings_WB_C" (`GameplayStatics.GetPlayerController` 0)))
      (set `self.Option WB` _returnvalue)))
  (`UserWidget.AddToViewport` (`self.Option WB`) 0))